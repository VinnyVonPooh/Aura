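; Gameplay ability for a melee attack that turns the avatar toward its combat target and plays a randomly chosen attack montage.
; Montages and their tags come from the avatar through combat interface calls, and the ability waits for the gameplay event matching the selected tag.
; On that event it damages live players in a small sphere around the tag's combat socket, then ends.
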(event Ability|EventActivateAbility
  (bind _returnvalue (Ability|GetAvatarActorfromActorInfo))
  (bind _returnvalue_2 (Ability|GetAvatarActorfromActorInfo))
  (bind _returnvalue_3 (Class|EnemyInterface|GetCombatTarget(Message) _returnvalue_2))
  (bind _ascombat_interface (Utilities|Casting|CastToCombatInterface _returnvalue_2)
    (:then
      (Class|CombatInterface|UpdateFacingTarget _ascombat_interface (Transformation|GetActorLocation _returnvalue_3))
      (bind (_montage _montagetag) (CallFunction|GetRandomMontageandTag))
      (|PlayMontageandWaitProxy "None" _montage 1.0 "None" true 1.0 0.0 false
        (:then
          (Ability|Tasks|WaitGameplayEvent _montagetag 0
            (:EventReceived
              (bind _returnvalue_4 (Class|CombatInterface|GetCombatSocketLocation(Message) _returnvalue _montagetag))
              (bind _outoverlappingactors (Class|AuraAbilitySystemLibrary|GetLivePlayersWithinRadius _returnvalue (Utilities|Array|MakeArray _returnvalue) 45.0 _returnvalue_4))
              (for _array_element _outoverlappingactors
                (Class|AuraDamageGameplayAbility|CauseDamage _array_element)))))))
    (:CastFailed
      _))
  (Ability|EndAbility))

(event Ability|EventOnEndAbility
  (params (bWasCancelled :type Boolean)))

(fn GetRandomMontageandTag
  (bind _returnvalue (Class|CombatInterface|GetAttackMontages(Message) (Ability|GetAvatarActorfromActorInfo)))
  (if (> (Utilities|Array|Length _returnvalue) 0)
    (return (.Montage (Utilities|Struct|BreakTaggedMontage (Utilities|Array|Get(acopy) _returnvalue (Math|Random|RandomIntegerinRange 0 (- (Utilities|Array|Length _returnvalue) 1))))) (.MontageTag (Utilities|Struct|BreakTaggedMontage (Utilities|Array|Get(acopy) _returnvalue (Math|Random|RandomIntegerinRange 0 (- (Utilities|Array|Length _returnvalue) 1))))))))