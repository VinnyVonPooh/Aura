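; Channeled lightning gameplay ability that chains a beam from the cursor target to additional targets while input is held.
; A montage event locks movement, starts ShockLoop cues and runs a looping timer that pays mana and applies lightning damage.
; Release (after a minimum time), empty mana or primary target death ends it, committing cooldown and applying stun-capable damage effects.
; Secondary deaths only drop that link, using stored per-target cue parameters.
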(event Custom|DamageAndCost
  ;[0.15 0.15 0.15 0.5] Тратим ману
  (bind _returnvalue (Ability|CommitAbilityCost false))
  (if _returnvalue
    (CallFunction|ApplyDamage)
    (else
      ;[0.15 0.15 0.15 0.5] Если маны больше нет
      (CallFunction|PreparetoEndAbility)
      (Ability|EndAbility))))

(event Ability|EventActivateAbility
  (CallFunction|InforceImplementsCombatInterface)
  ;[0.15 0.15 0.15 0.5] Хранение данных - то что под курсором
  (bind _datahandle (|TargetDataUnderMouse)
    (:ValidData
      (Class|AuraBeamSpell|StoreMouseDataInfo (Ability|TargetData|GetHitResultfromTargetData _datahandle))
      (Class|AuraBeamSpell|StoreOwnerPlayerVariables)
      (Utilities|FlowControl|Sequence
        (:then_0
          (Variables|/Script/Engine.PlayerController|SetbShowMouseCursor (Variables|Default|GetOwnerPlayerController) false)
          (CallFunction|UpdateFacingTarget)
          (GameplayCue|ExecuteGameplayCue :GameplayCueTag "(TagName=\"GameplayCue.ShockBurst\")")
          (|PlayMontageandWaitProxy "None" (Variables|Default|GetMontage_Electricute) 1.0 "None" false 1.0 0.0 false
            (:then
              (Ability|Tasks|WaitGameplayEvent "(TagName=\"Event.Montage.Electrocute\")" 0
                (:EventReceived
                  (CallFunction|InShockLoop)
                  (CallFunction|SpawnElectricBeam)
                  (bind _returnvalue (Utilities|Time|SetTimerbyEvent (delegate Custom|DamageAndCost) (Variables|Default|GetDamageDeltaTime) true))
                  (Variables|Default|SetDamageAndCostTimer _returnvalue))))))
        (:then_1
          (bind _timeheld (Ability|Tasks|WaitInputRelease false)
            (:OnRelease
              ;[0.15 0.15 0.15 0.5] Если удерживали мышку не долго, даём ещё немного поиграть эффекту
              (bind _output_get (Variables|Default|SetTime%20Held _timeheld))
              (if (< _output_get (Variables|Default|GetMinSpellTime))
                (Utilities|FlowControl|Delay (- (Variables|Default|GetMinSpellTime) (Variables|Default|GetTime%20Held))))
              (CallFunction|PreparetoEndAbility)
              (Ability|EndAbility))))))))

(event Ability|EventOnEndAbility
  (params (bWasCancelled :type Boolean)))

(event EventPrimaryTargetDied
  (params (DeadActor :type Actor%20Object%20Reference))
  ;[0.15 0.15 0.15 0.5] Если первичная цель умерла
  (GameplayCue|RemoveGameplayCueOnActor(Looping) DeadActor "(TagName=\"GameplayCue.ShockLoop\")" (Variables|Default|GetFirstTargetCueParams))
  (CallFunction|PreparetoEndAbility)
  (Ability|EndAbility))

(event EventAdditionalTargetDied
  (params (DeadActor :type Actor%20Object%20Reference))
  ;[0.15 0.15 0.15 0.5] Если цель в цепочке умерла
  (CallFunction|RemoveShockLoopCuetoAdditionalTarget DeadActor)
  (Utilities|Array|RemoveItem (Variables|Default|GetAdditionalTargets) DeadActor))

(fn InforceImplementsCombatInterface
  (if (not (Utilities|DoesObjectImplementInterface (Ability|GetAvatarActorfromActorInfo) "/Script/Aura.CombatInterface"))
    (Ability|EndAbility)))

(fn PreparetoEndAbility
  (Ability|CommitAbilityCooldown false)
  (Variables|/Script/Engine.PlayerController|SetbShowMouseCursor (Variables|Default|GetOwnerPlayerController) true)
  (Class|CombatInterface|SetinShockLoop(Message) (Ability|GetAvatarActorfromActorInfo) false)
  (Pawn|Components|CharacterMovement|SetMovementMode (Variables|/Script/Engine.Character|GetCharacterMovement (Variables|Default|GetOwnerCharacter)) "MOVE_Walking" 0)
  (GameplayCue|RemoveGameplayCueOnActor(Looping) (Variables|Default|GetCueActor) "(TagName=\"GameplayCue.ShockLoop\")" (Variables|Default|GetFirstTargetCueParams))
  (Utilities|Time|ClearandInvalidateTimerbyHandle (Variables|Default|GetDamageAndCostTimer))
  (if (Variables|Default|GetFirstTargetImplementsInterface)
    ;[0.15 0.15 0.15 0.5] Логика для стана
    (Class|AuraAbilitySystemLibrary|ApplyDamageEffect (Class|AuraDamageGameplayAbility|MakeDamageEffectParamsfromClassDefaults (Variables|Default|GetMouseHitActor)))
    (for _array_element (Variables|Default|GetAdditionalTargets)
      (CallFunction|RemoveShockLoopCuetoAdditionalTarget _array_element)
      (Class|AuraAbilitySystemLibrary|ApplyDamageEffect (Class|AuraDamageGameplayAbility|MakeDamageEffectParamsfromClassDefaults _array_element))))
  (Utilities|Array|Clear (Variables|Default|GetAdditionalTargets))
  (Utilities|Map|Clear (Variables|Default|GetAdditionalTargetsToCueParams))
  (Variables|Default|SetMouseHitActor 0)
  (Variables|Default|SetFirstTargetImplementsInterface false)
  (Variables|Default|SetTime%20Held 0.0))

(fn InShockLoop
  (Class|CombatInterface|SetinShockLoop(Message) (Ability|GetAvatarActorfromActorInfo) true)
  (Pawn|Components|CharacterMovement|DisableMovement (Variables|/Script/Engine.Character|GetCharacterMovement (Variables|Default|GetOwnerCharacter))))

(fn UpdateFacingTarget
  (Class|CombatInterface|UpdateFacingTarget(Message) (Ability|GetAvatarActorfromActorInfo) (Variables|Default|GetMouseHitLocation)))

(fn SpawnElectricBeam
  (Class|AuraBeamSpell|TraceFirstTarget (Variables|Default|GetMouseHitLocation))
  (bind _returnvalue (Class|CombatInterface|GetWeapon(Message) (Variables|Default|GetOwnerCharacter)))
  (Variables|Default|SetFirstTargetCueParams (Ability|GameplayCue|MakeGameplayCueParameters :Location (Variables|Default|GetMouseHitLocation) :SourceObject (Variables|Default|GetMouseHitActor) :TargetAttachComponent _returnvalue))
  (bind _output_get (Variables|Default|SetFirstTargetImplementsInterface (Utilities|DoesObjectImplementInterface (Variables|Default|GetMouseHitActor) "/Script/Aura.CombatInterface")))
  (if _output_get
    (Variables|Default|SetCueActor (Variables|Default|GetMouseHitActor))
    (else
      (Variables|Default|SetCueActor (Ability|GetAvatarActorfromActorInfo))))
  (GameplayCue|AddGameplayCueOnActor(Looping) (Variables|Default|GetCueActor) "(TagName=\"GameplayCue.ShockLoop\")" (Variables|Default|GetFirstTargetCueParams))
  (if (Variables|Default|GetFirstTargetImplementsInterface)
    (bind _outadditionaltargets (Class|AuraBeamSpell|StoreAdditionalTargets))
    (bind _output_get_2 (Variables|Default|SetAdditionalTargets _outadditionaltargets))
    (for _array_element _output_get_2
      (CallFunction|AddShockLoopCuetoAdditionalTarget _array_element))))

(fn AddShockLoopCuetoAdditionalTarget
  (params (AdditionalTarget :type Actor%20Object%20Reference))
  (bind _mousehitactor (Variables|Default|GetMouseHitActor))
  (bind _returnvalue (Transformation|GetActorLocation AdditionalTarget))
  (bind _rootcomponent (Variables|/Script/Engine.Actor|GetRootComponent _mousehitactor))
  (bind _returnvalue_2 (Ability|GameplayCue|MakeGameplayCueParameters :Location _returnvalue :SourceObject AdditionalTarget :TargetAttachComponent _rootcomponent))
  (Utilities|Map|Add (Variables|Default|GetAdditionalTargetsToCueParams) AdditionalTarget _returnvalue_2)
  (GameplayCue|AddGameplayCueOnActor(Looping) AdditionalTarget "(TagName=\"GameplayCue.ShockLoop\")" _returnvalue_2))

(fn RemoveShockLoopCuetoAdditionalTarget
  (params (AdditionalTarget :type Actor%20Object%20Reference))
  (bind _additionaltargetstocueparams (Variables|Default|GetAdditionalTargetsToCueParams))
  (bind (_value _returnvalue) (Utilities|Map|Find _additionaltargetstocueparams AdditionalTarget))
  (if _returnvalue
    (GameplayCue|RemoveGameplayCueOnActor(Looping) AdditionalTarget "(TagName=\"GameplayCue.ShockLoop\")" _value)))

(fn ApplyDamage
  (CallFunction|ApplyDamageSingleTarget (Variables|Default|GetMouseHitActor))
  (for _array_element (Variables|Default|GetAdditionalTargets)
    (CallFunction|ApplyDamageSingleTarget _array_element)))

(fn ApplyDamageSingleTarget
  (params (InActor :type Actor%20Object%20Reference))
  (bind _returnvalue (Ability|GetAbilitySystemComponent InActor))
  (Utilities|IsValid InActor
    (:Is%20Valid
      (bind _output_get (LocalVariables|SetASC (Ability|GetAbilitySystemComponentfromActorInfo)))
      (Utilities|IsValid _output_get
        (:Is%20Valid
          (bind _returnvalue_2 (Ability|GameplayEffect|AssignTagSetbyCallerMagnitude (GameplayEffects|MakeOutgoingSpec (LocalVariables|GetASC) (Variables|Default|GetDamageEffectClass) (Math|Conversions|ToFloat(Integer) (Ability|GetAbilityLevel)) (GameplayEffects|MakeEffectContext (LocalVariables|GetASC))) "(TagName=\"Damage.Lightning\")" (Class|AuraDamageGameplayAbility|GetDamageatLevel)))
          (Utilities|IsValid _returnvalue
            (:Is%20Valid
              (GameplayEffects|ApplyGameplayEffectSpecToSelf _returnvalue _returnvalue_2))))))))