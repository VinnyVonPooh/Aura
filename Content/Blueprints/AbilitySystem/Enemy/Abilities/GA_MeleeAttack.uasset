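; Enemy melee attack gameplay ability that faces the combat target and plays a random tagged attack montage.
; When the montage's gameplay event fires, it samples the matching combat socket and damages non-friendly live players within a small radius of it.
; A hit triggers a melee impact gameplay cue tagged with the montage, and the ability ends after the event or if the montage is interrupted or cancelled.
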(event Ability|EventActivateAbility
  (bind _returnvalue (Ability|GetAvatarActorfromActorInfo))
  (bind _returnvalue_2 (Ability|GetAvatarActorfromActorInfo))
  (Variables|Default|SetHasHitTarget false)
  (bind _returnvalue_3 (Class|EnemyInterface|GetCombatTarget(Message) _returnvalue))
  (Variables|Default|SetCombatTarget _returnvalue_3)
  (bind _ascombat_interface (Utilities|Casting|CastToCombatInterface _returnvalue)
    (:then
      (Class|CombatInterface|UpdateFacingTarget _ascombat_interface (Transformation|GetActorLocation (Variables|Default|GetCombatTarget)))
      (bind _returnvalue_4 (Class|CombatInterface|GetAttackMontages(Message) (Ability|GetAvatarActorfromActorInfo)))
      (Variables|Default|SetTaggedMontage (Class|AuraDamageGameplayAbility|GetRandomTaggedMontagefromArray _returnvalue_4))
      (|PlayMontageandWaitProxy "None" (.montage (Variables|Default|GetTaggedMontage)) 1.0 "None" true 1.0 0.0 false
        (:then
          (Ability|Tasks|WaitGameplayEvent (.montagetag (Variables|Default|GetTaggedMontage)) 0
            (:EventReceived
              (bind _returnvalue_5 (Class|CombatInterface|GetCombatSocketLocation(Message) _returnvalue_2 (.sockettag (Variables|Default|GetTaggedMontage))))
              (bind _output_get (Variables|Default|SetHitLocation _returnvalue_5))
              (bind _outoverlappingactors (Class|AuraAbilitySystemLibrary|GetLivePlayersWithinRadius _returnvalue_2 (Utilities|Array|MakeArray _returnvalue_2) 45.0 _output_get))
              (for _array_element _outoverlappingactors
                (if (Class|AuraAbilitySystemLibrary|IsNotFriend (Ability|GetAvatarActorfromActorInfo) _array_element)
                  (Class|AuraAbilitySystemLibrary|ApplyDamageEffect (Class|AuraDamageGameplayAbility|MakeDamageEffectParamsfromClassDefaults _array_element))
                  (Variables|Default|SetHasHitTarget true)))
              (if (Variables|Default|GetHasHitTarget)
                (Class|GameplayAbility|ExecuteGameplayCuewithParams "(TagName=\"GameplayCue.MeleeImpact\")" (Ability|GameplayCue|MakeGameplayCueParameters :AggregatedSourceTags (GameplayTags|MakeGameplayTagContainerfromTag (.montagetag (Variables|Default|GetTaggedMontage))) :Location (Variables|Default|GetHitLocation) :EffectCauser (Ability|GetAvatarActorfromActorInfo) :SourceObject (Variables|Default|GetCombatTarget)))))))
        (:OnInterrupted
          _)
        (:OnCancelled
          _)))
    (:CastFailed
      _))
  (Ability|EndAbility))

(event Ability|EventOnEndAbility
  (params (bWasCancelled :type Boolean)))